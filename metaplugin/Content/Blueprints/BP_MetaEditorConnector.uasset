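; Bridge between a Pixel Streaming web client and the game, handling remote JSON commands.
; On BeginPlay it binds to the player controller's PixelStreamingInput, parses each message into a request struct and routes it by command name.
; Handlers change resolution, run console commands, set volume, toggle screen messages or cursor, and return command or response history.
; SendResponse echoes the request with a timestamped response, prints it and records it.
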(event Custom|OnInput
  (params (Descriptor :type String))
  (CallFunction|ParseInput Descriptor))

(event EventBeginPlay
  (bind _returnvalue (Game|GetPlayerController 0))
  (bind _returnvalue_2 (Actor|GetComponentbyClass _returnvalue "/Script/PixelStreaming.PixelStreamingInput"))
  (Utilities|IsValid _returnvalue_2
    (:Is%20Valid
      (EventDispatchers|BindEventtoOnInputEvent _returnvalue_2 (delegate Custom|OnInput)))))

(fn ConstructionScript)

(fn ParseCommand
  (params (JsonObject :type Meta%20Editor%20Json%20Object%20Structure))
  (if (Math|Boolean|ANDBoolean (Class|MetaEditorLibrary|JsonHasField JsonObject "command") (Class|MetaEditorLibrary|JsonHasField JsonObject "request") (Class|MetaEditorLibrary|JsonHasField JsonObject "verification_id") (Class|MetaEditorLibrary|JsonHasField JsonObject "initiator"))
    (return (Utilities|Struct|MakeBP_MetaEditorJsonRequest (Class|MetaEditorLibrary|ToString(JsonValue) (Class|MetaEditorLibrary|ToJsonValue(JsonObject) JsonObject "verification_id")) (Class|MetaEditorLibrary|ToString(JsonValue) (Class|MetaEditorLibrary|ToJsonValue(JsonObject) JsonObject "command")) (Class|MetaEditorLibrary|ToString(JsonValue) (Class|MetaEditorLibrary|ToJsonValue(JsonObject) JsonObject "initiator")) (Class|MetaEditorLibrary|ToObject(JsonValue) (Class|MetaEditorLibrary|ToJsonValue(JsonObject) JsonObject "request"))))
    (else
      (return (Utilities|Struct|MakeBP_MetaEditorJsonRequest "" "" "" "()")))))

(fn SendEmptyResponse
  (CallFunction|SendResponse (Utilities|Struct|MakeBP_MetaEditorJsonRequest "" "" "ue" "()") (Class|MetaEditorLibrary|JsonMakeField (Class|MetaEditorLibrary|JsonMakeField (Class|MetaEditorLibrary|JsonMake) "time" (Class|MetaEditorLibrary|JsonMakeString (CallFunction|GetUTCTimeNow))) "body" (Class|MetaEditorLibrary|JsonMakeNull))))

(fn SendResponse
  (params (request :type BP%20Meta%20Editor%20Json%20Request%20Structure) (response :type Meta%20Editor%20Json%20Object%20Structure))
  (bind (_verificationid _command _caller _request) (Utilities|Struct|BreakBP_MetaEditorJsonRequest request))
  (bind _returnvalue (Class|MetaEditorLibrary|JsonMakeObject response))
  (bind _returnvalue_2 (Class|MetaEditorLibrary|JsonMake))
  (bind _returnvalue_3 (Class|MetaEditorLibrary|JsonMakeString _caller))
  (bind _returnvalue_4 (Class|MetaEditorLibrary|JsonMakeObject _request))
  (bind _returnvalue_5 (Class|MetaEditorLibrary|JsonMakeString _command))
  (bind _returnvalue_6 (Class|MetaEditorLibrary|JsonMakeString _verificationid))
  (bind _returnvalue_7 (Class|MetaEditorLibrary|JsonMakeField _returnvalue_2 "verification_id" _returnvalue_6))
  (bind _returnvalue_8 (Class|MetaEditorLibrary|JsonMakeField _returnvalue_7 "initiator" _returnvalue_3))
  (bind _returnvalue_9 (Class|MetaEditorLibrary|JsonMakeField _returnvalue_8 "command" _returnvalue_5))
  (bind _returnvalue_10 (Class|MetaEditorLibrary|JsonMakeField _returnvalue_9 "request" _returnvalue_4))
  (bind _returnvalue_11 (Class|MetaEditorLibrary|JsonMakeField _returnvalue_10 "response" _returnvalue))
  (bind _returnvalue_12 (Class|MetaEditorLibrary|ToString(JsonObject) _returnvalue_11))
  (Class|PixelStreamingInput|SendPixelStreamingResponse (Actor|GetComponentbyClass (Game|GetPlayerController 0) "/Script/PixelStreaming.PixelStreamingInput") _returnvalue_12)
  (Utilities|Array|Add (Variables|Default|GetCallbacksHistory) (Class|MetaEditorLibrary|JsonMakeObject _returnvalue_11))
  (Development|PrintString _returnvalue_12))

(fn ConsoleCommand
  (params (request :type BP%20Meta%20Editor%20Json%20Request%20Structure))
  (bind _request (Utilities|Struct|BreakBP_MetaEditorJsonRequest request))
  (bind _returnvalue (Class|MetaEditorLibrary|ToJsonValue(JsonObject) _request "body"))
  (bind _returnvalue_2 (Class|MetaEditorLibrary|ToObject(JsonValue) _returnvalue))
  (if (Class|MetaEditorLibrary|JsonHasField _request "body")
    (if (Class|MetaEditorLibrary|JsonHasField _returnvalue_2 "command")
      (Development|ExecuteConsoleCommand (Class|MetaEditorLibrary|ToString(JsonValue) (Class|MetaEditorLibrary|ToJsonValue(JsonObject) _returnvalue_2 "command")) 0)
      (CallFunction|SendResponse request (Class|MetaEditorLibrary|JsonMakeField (Class|MetaEditorLibrary|JsonMakeField (Class|MetaEditorLibrary|JsonMake) "time" (Class|MetaEditorLibrary|JsonMakeString (CallFunction|GetUTCTimeNow))) "body" _returnvalue)))))

(fn GetUTCTimeNow
  (bind _returnvalue (Math|DateTime|UTCNow))
  (bind (_year _month _day _hour _minute _second) (Math|DateTime|BreakDateTime _returnvalue))
  (return (Utilities|String|Append (Utilities|String|ToString(Integer) _year) "-" (Utilities|String|ToString(Text) (Utilities|Text|ToText(Integer) _month false true 2 2)) "-" (Utilities|String|ToString(Text) (Utilities|Text|ToText(Integer) _day false true 2 2)) "T" (Utilities|String|ToString(Text) (Utilities|Text|ToText(Integer) _hour false true 2 2)) ":" (Utilities|String|ToString(Text) (Utilities|Text|ToText(Integer) _minute false true 2 2)) ":" (Utilities|String|ToString(Text) (Utilities|Text|ToText(Integer) _second false true 2 2)) "Z")))

(fn ResolutionChange
  (params (request :type BP%20Meta%20Editor%20Json%20Request%20Structure))
  (bind _request (Utilities|Struct|BreakBP_MetaEditorJsonRequest request))
  (bind _returnvalue (Class|MetaEditorLibrary|ToJsonValue(JsonObject) _request "body"))
  (bind _returnvalue_2 (Class|MetaEditorLibrary|ToObject(JsonValue) _returnvalue))
  (bind _returnvalue_3 (Class|MetaEditorLibrary|ToObject(JsonValue) _returnvalue))
  (bind _returnvalue_4 (Class|MetaEditorLibrary|ToJsonValue(JsonObject) _returnvalue_2 "height"))
  (bind _returnvalue_5 (Class|MetaEditorLibrary|ToJsonValue(JsonObject) _returnvalue_3 "width"))
  (bind _returnvalue_6 (Class|MetaEditorLibrary|ToInteger(JsonValue) _returnvalue_4))
  (bind _returnvalue_7 (Class|MetaEditorLibrary|ToInteger(JsonValue) _returnvalue_5))
  (if (Class|MetaEditorLibrary|JsonHasField _request "body")
    (if (and (Class|MetaEditorLibrary|JsonHasField _returnvalue_3 "width") (Class|MetaEditorLibrary|JsonHasField _returnvalue_2 "height"))
      (Development|ExecuteConsoleCommand (Utilities|String|Append "PixelStreaming.Capturer.UseBackBufferSize 0" "") 0)
      (Development|ExecuteConsoleCommand (Utilities|String|Append "PixelStreaming.WebRTC.DisableResolutionChange 0" "") 0)
      (Development|ExecuteConsoleCommand (Utilities|String|Append "PixelStreaming.Capturer.CaptureSize " (Utilities|String|ToString(Integer) _returnvalue_7) "x" (Utilities|String|ToString(Integer) _returnvalue_6)) 0)
      (bind _returnvalue_8 (Settings|GetGameUserSettings))
      (Class|GameUserSettings|SetFullscreenMode _returnvalue_8 "Windowed")
      (Class|GameUserSettings|SetScreenResolution _returnvalue_8 (Utilities|Struct|MakeIntPoint _returnvalue_7 _returnvalue_6))
      (Class|GameUserSettings|ApplySettings _returnvalue_8 false)
      (CallFunction|SendResponse request (Class|MetaEditorLibrary|JsonMakeField (Class|MetaEditorLibrary|JsonMakeField (Class|MetaEditorLibrary|JsonMake) "time" (Class|MetaEditorLibrary|JsonMakeString (CallFunction|GetUTCTimeNow))) "body" _returnvalue)))))

(fn ChangeSound
  (params (request :type BP%20Meta%20Editor%20Json%20Request%20Structure))
  (bind _request (Utilities|Struct|BreakBP_MetaEditorJsonRequest request))
  (bind _returnvalue (Class|MetaEditorLibrary|ToJsonValue(JsonObject) _request "body"))
  (bind _returnvalue_2 (Class|MetaEditorLibrary|ToObject(JsonValue) _returnvalue))
  (if (and (Class|MetaEditorLibrary|JsonHasField _request "body") (Class|MetaEditorLibrary|JsonHasField _returnvalue_2 "volume"))
    (Audio|SetSoundMixClassOverride "/Game/CarConfigurator/Shared/Audio/AMP_SoundMix.AMP_SoundMix" "/Game/CarConfigurator/Shared/Audio/AMP_Master.AMP_Master" (Class|MetaEditorLibrary|ToFloat(JsonValue) (Class|MetaEditorLibrary|ToJsonValue(JsonObject) _returnvalue_2 "volume")) 1.0 1.0 true)
    (CallFunction|SendResponse request (Class|MetaEditorLibrary|JsonMakeField (Class|MetaEditorLibrary|JsonMakeField (Class|MetaEditorLibrary|JsonMake) "time" (Class|MetaEditorLibrary|JsonMakeString (CallFunction|GetUTCTimeNow))) "body" _returnvalue))))

(fn DebugMode
  (params (request :type BP%20Meta%20Editor%20Json%20Request%20Structure))
  (bind _request (Utilities|Struct|BreakBP_MetaEditorJsonRequest request))
  (bind _returnvalue (Class|MetaEditorLibrary|ToJsonValue(JsonObject) _request "body"))
  (bind _returnvalue_2 (Class|MetaEditorLibrary|ToObject(JsonValue) _returnvalue))
  (if (and (Class|MetaEditorLibrary|JsonHasField _request "body") (Class|MetaEditorLibrary|JsonHasField _returnvalue_2 "mode"))
    (switch string (Class|MetaEditorLibrary|ToString(JsonValue) (Class|MetaEditorLibrary|ToJsonValue(JsonObject) _returnvalue_2 "mode"))
      (:on
        (Development|ExecuteConsoleCommand "ENABLEALLSCREENMESSAGES" 0))
      (:off
        (Development|ExecuteConsoleCommand "DISABLEALLSCREENMESSAGES" 0)))
    (CallFunction|SendResponse request (Class|MetaEditorLibrary|JsonMakeField (Class|MetaEditorLibrary|JsonMakeField (Class|MetaEditorLibrary|JsonMake) "time" (Class|MetaEditorLibrary|JsonMakeString (CallFunction|GetUTCTimeNow))) "body" _returnvalue))))

(fn Cursor
  (params (request :type BP%20Meta%20Editor%20Json%20Request%20Structure))
  (bind _request (Utilities|Struct|BreakBP_MetaEditorJsonRequest request))
  (bind _returnvalue (Class|MetaEditorLibrary|ToJsonValue(JsonObject) _request "body"))
  (bind _returnvalue_2 (Class|MetaEditorLibrary|ToObject(JsonValue) _returnvalue))
  (if (and (Class|MetaEditorLibrary|JsonHasField _request "body") (Class|MetaEditorLibrary|JsonHasField _returnvalue_2 "enabled"))
    (if (Class|MetaEditorLibrary|ToBoolean(JsonValue) (Class|MetaEditorLibrary|ToJsonValue(JsonObject) _returnvalue_2 "enabled"))
      (Variables|/Script/Engine.PlayerController|SetbShowMouseCursor (Game|GetPlayerController 0) true)
      (else
        (Variables|/Script/Engine.PlayerController|SetbShowMouseCursor (Game|GetPlayerController 0) false)))
    (CallFunction|SendResponse request (Class|MetaEditorLibrary|JsonMakeField (Class|MetaEditorLibrary|JsonMakeField (Class|MetaEditorLibrary|JsonMake) "time" (Class|MetaEditorLibrary|JsonMakeString (CallFunction|GetUTCTimeNow))) "body" _returnvalue))))

(fn CallbacksHistory
  (params (request :type BP%20Meta%20Editor%20Json%20Request%20Structure))
  (bind _request (Utilities|Struct|BreakBP_MetaEditorJsonRequest request))
  (if (Class|MetaEditorLibrary|JsonHasField _request "body")
    (if (Class|MetaEditorLibrary|ToBoolean(JsonValue) (Class|MetaEditorLibrary|ToJsonValue(JsonObject) _request "body"))
      (CallFunction|SendResponse request (Class|MetaEditorLibrary|JsonMakeField (Class|MetaEditorLibrary|JsonMakeField (Class|MetaEditorLibrary|JsonMake) "time" (Class|MetaEditorLibrary|JsonMakeString (CallFunction|GetUTCTimeNow))) "body" (Class|MetaEditorLibrary|JsonMakeArray (Variables|Default|GetCallbacksHistory)))))))

(fn CommandsHistory
  (params (request :type BP%20Meta%20Editor%20Json%20Request%20Structure))
  (bind _request (Utilities|Struct|BreakBP_MetaEditorJsonRequest request))
  (if (Class|MetaEditorLibrary|JsonHasField _request "body")
    (if (Class|MetaEditorLibrary|ToBoolean(JsonValue) (Class|MetaEditorLibrary|ToJsonValue(JsonObject) _request "body"))
      (CallFunction|SendResponse request (Class|MetaEditorLibrary|JsonMakeField (Class|MetaEditorLibrary|JsonMakeField (Class|MetaEditorLibrary|JsonMake) "time" (Class|MetaEditorLibrary|JsonMakeString (CallFunction|GetUTCTimeNow))) "body" (Class|MetaEditorLibrary|JsonMakeArray (Variables|Default|GetCommandsHistory)))))))

(fn CommandNotFound
  (params (request :type BP%20Meta%20Editor%20Json%20Request%20Structure))
  (if (Utilities|Enum|NotEqual(Enum) (.Command (Utilities|Struct|BreakBP_MetaEditorJsonRequest request)) "")
    (CallFunction|SendResponse request (Class|MetaEditorLibrary|JsonMakeField (Class|MetaEditorLibrary|JsonMakeField (Class|MetaEditorLibrary|JsonMakeField (Class|MetaEditorLibrary|JsonMakeField (Class|MetaEditorLibrary|JsonMake) "time" (Class|MetaEditorLibrary|JsonMakeString (CallFunction|GetUTCTimeNow))) "body" (Class|MetaEditorLibrary|JsonMakeNull)) "error" (Class|MetaEditorLibrary|JsonMakeBool true)) "message" (Class|MetaEditorLibrary|JsonMakeString "command not found")))))

(fn ParseInput
  (params (JsonString :type String))
  (bind _returnvalue (Class|MetaEditorLibrary|ToJsonObject(String) JsonString))
  (Development|PrintString JsonString)
  (bind _request (CallFunction|ParseCommand _returnvalue))
  (bind _outrequest (Utilities|ChangeCommand _request)
    (:resolution_change
      (CallFunction|ResolutionChange _outrequest))
    (:console_command
      (CallFunction|ConsoleCommand _outrequest))
    (:debug_mode
      (CallFunction|DebugMode _outrequest))
    (:user_sound
      (CallFunction|ChangeSound _outrequest))
    (:cursor
      (CallFunction|Cursor _outrequest))
    (:commands_history
      (CallFunction|CommandsHistory _outrequest))
    (:callbacks_history
      (CallFunction|CallbacksHistory _outrequest))
    (:default
      (CallFunction|CommandNotFound _outrequest)))
  (Utilities|Array|Add (Variables|Default|GetCommandsHistory) (Class|MetaEditorLibrary|JsonMakeObject _returnvalue)))